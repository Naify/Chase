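; BP_ChaseGameMode is the game mode that tracks NPC deaths and ends the game when the last NPC dies.
; NpcDied uses GameSettings.NPCNumberToSpawn as the remaining count, decrementing it directly until it reaches one, then calling EndGame on the next death.
; EndGame shows the WBP_GameEnd widget, enables the mouse cursor and switches the first player controller to Game and UI input.
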(event `self.ReceiveBeginPlay`)

(event `NpcDied`
  (bind (_playersspeed _npcspeed _npcnumbertospawn) (break `GameSettings` (`self.GameSettings`)))
  (if (<= _npcnumbertospawn 1)
    (`self.EndGame`)
    (else
      (`/Engine/EditorBlueprintResources/StandardMacros.DecrementInt` _npcnumbertospawn))))

(event `EndGame`
  (bind _returnvalue (`GameplayStatics.GetPlayerController` 0))
  (bind _returnvalue_2 (`|CreateWidget` "/Game/ChaseGame/UI/Menu/WBP_GameEnd.WBP_GameEnd_C"))
  (`UserWidget.AddToPlayerScreen` _returnvalue_2 0)
  (set `PlayerController.bShowMouseCursor` true _returnvalue)
  (`WidgetBlueprintLibrary.SetInputMode_GameAndUIEx` _returnvalue null))

(fn `UserConstructionScript`)
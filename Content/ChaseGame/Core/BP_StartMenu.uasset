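; BP_StartMenu runs the start menu of ChaseGame and launches the play level.
; On BeginPlay it creates the WBP_GameStart widget, binds its StartPressed event, and switches to UI-only input with a visible cursor.
; When start is pressed, it stores the passed GameSettings in BP_ChaseGameInstance, then opens the level named by that instance's PlayLevelName.
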(event `self.ReceiveBeginPlay`
  (bind _returnvalue (`GameplayStatics.GetPlayerController` 0))
  (bind _returnvalue_2 (`|CreateWidget` "/Game/ChaseGame/UI/Menu/WBP_GameStart.WBP_GameStart_C"))
  (add `/Game/ChaseGame/UI/Menu/WBP_GameStart.StartPressed` _returnvalue_2 (delegate `Start`))
  (`UserWidget.AddToPlayerScreen` _returnvalue_2 0)
  (set `PlayerController.bShowMouseCursor` true _returnvalue)
  (`WidgetBlueprintLibrary.SetInputMode_UIOnlyEx` _returnvalue null))

(event `Start`
  (params (GameSettings :type "GameSettings Structure"))
  (bind _asbp_chase_game_instance (cast `/Game/ChaseGame/Core/BP_ChaseGameInstance` (`GameplayStatics.GetGameInstance`)))
  (set `ChaseGameInstance.GameSettings` GameSettings _asbp_chase_game_instance)
  (`GameplayStatics.OpenLevel` (`ChaseGameInstance.PlayLevelName` _asbp_chase_game_instance)))

(fn `UserConstructionScript`)
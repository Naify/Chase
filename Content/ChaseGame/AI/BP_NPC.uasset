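; BP_NPC is the chase game's NPC character, with health, a health bar and a ragdoll death.
; On BeginPlay it writes MovementRadius to the Blackboard and takes walk speed and max health from BP_ChaseGameMode's settings.
; ChaseHealthComponent events update the WBP_HealthBar widget, hidden at zero health.
; On death it ragdolls, disables movement, expires after a short lifespan and decrements the game mode's NPC count.
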(event `self.ReceiveBeginPlay`
  (bind _chasehealthcomponent (`self.ChaseHealthComponent`))
  (`BlackboardComponent.SetValueAsFloat` (`AIBlueprintHelperLibrary.GetBlackboard` null) "MovementRadius" (`self.MovementRadius`))
  ;[1 1 1] Because components beginplay() called before characters
  (`self.OnHealthChanged` (`ChaseHealthActorComponent.MaxHealth` (`self.ChaseHealthComponent`)))
  (add `ChaseHealthActorComponent.OnDeath` _chasehealthcomponent (`|CreateDelegate` :!event `OnDeath`))
  (add `ChaseHealthActorComponent.OnHealthChanged` _chasehealthcomponent (`|CreateDelegate` :!event `OnHealthChanged`))
  (bind _asbp_chase_game_mode (cast `/Game/ChaseGame/Core/BP_ChaseGameMode` (`GameplayStatics.GetGameMode`)))
  (bind (_playersspeed _npcspeed _npcnumbertospawn _playershotdistance _playershotdamage _npcmaxhealth) (break `GameSettings` (`ChaseGameMode.GameSettings` _asbp_chase_game_mode)))
  (set `CharacterMovementComponent.MaxWalkSpeed` _npcspeed (`self.CharacterMovement`))
  (set `ChaseHealthActorComponent.MaxHealth` _npcmaxhealth (`self.ChaseHealthComponent`)))

(event `self.ReceiveTick`
  (params (DeltaSeconds :type "Float (single-precision)")))

(event `OnDeath`
  (`PrimitiveComponent.SetCollisionProfileName` (`self.Mesh`) "Ragdoll" true)
  (`PrimitiveComponent.SetSimulatePhysics` (`self.Mesh`) true)
  (`CharacterMovementComponent.DisableMovement` (`self.CharacterMovement`))
  (`self.SetLifeSpan` 2.0)
  (bind _asbp_chase_game_mode (cast `/Game/ChaseGame/Core/BP_ChaseGameMode` (`GameplayStatics.GetGameMode`)))
  (`/Engine/EditorBlueprintResources/StandardMacros.DecrementInt` (`/Game/ChaseGame/Core/BP_ChaseGameMode.CurrentNPCNumber` _asbp_chase_game_mode)))

(event `OnHealthChanged`
  (params (Health :type "Float (single-precision)"))
  (bind _healthbar (`self.HealthBar`))
  (bind _aswbp_health_bar (cast `/Game/ChaseGame/UI/NPCWidget/WBP_HealthBar` (`WidgetComponent.GetUserWidgetObject` _healthbar)))
  (bind _output_get (set `/Game/ChaseGame/UI/NPCWidget/WBP_HealthBar.Health` (/ Health (`ChaseHealthActorComponent.MaxHealth` (`self.ChaseHealthComponent`))) _aswbp_health_bar))
  (if (== _output_get 0.0)
    (`SceneComponent.SetHiddenInGame` _healthbar true false)))

(fn `UserConstructionScript`)